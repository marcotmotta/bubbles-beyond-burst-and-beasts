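; Homing acid projectile, apparently fired by a tower, that damages and corrodes enemies on contact.
; On BeginPlay it homes on HomingTargetComponent and destroys itself after a fixed lifetime, or on Tick if that target becomes invalid.
; Sphere overlap with an actor tagged Enemy applies damage and a hit sound, then calls Corrode on BP_Enemy for timed corrosion and destroys the projectile.
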(event OnComponentBeginOverlap(Sphere)
  (params (OverlappedComponent :type Primitive%20Component%20Object%20Reference) (OtherActor :type Actor%20Object%20Reference) (OtherComp :type Primitive%20Component%20Object%20Reference) (OtherBodyIndex :type Integer) (bFromSweep :type Boolean) (SweepResult :type Hit%20Result%20Structure%20%28by%20ref%29))
  (if (Actor|ActorHasTag OtherActor "Enemy")
    (Game|Damage|ApplyDamage OtherActor 1e+01 0 0)
    (Audio|PlaySoundatLocation "/Game/Assets/SFXs/Gorfada_Hit_1.Gorfada_Hit_1" (Transformation|GetActorLocation) "0, 0, 0" 1.0 1.0 0.0 0 0 0 0)
    (bind _asbp_enemy (Utilities|Casting|CastToBP_Enemy OtherActor))
    (Default|Corrode _asbp_enemy 3.0 2e+01)
    (Actor|DestroyActor)))

(event EventBeginPlay
  (Variables|/Script/Engine.ProjectileMovementComponent|SetHomingTargetComponent (Variables|Components|GetProjectileMovement) (Variables|Components|GetHoming%20Target%20Component))
  (Utilities|FlowControl|Delay 1e+01)
  (Actor|DestroyActor))

(event Collision|EventActorBeginOverlap
  (params (OtherActor :type Actor%20Object%20Reference)))

(event EventTick
  (params (DeltaSeconds :type Float%20%28single-precision%29))
  (Utilities|IsValid (Variables|Components|GetHoming%20Target%20Component)
    (:Is%20Not%20Valid
      (Actor|DestroyActor))))

(fn ConstructionScript)
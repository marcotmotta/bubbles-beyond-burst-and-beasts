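; BP_AcidTower is a tower that automatically fires homing acid projectiles at enemy-tagged actors.
; The Radius component locks onto the first enemy to enter and, when that target leaves, picks the nearest overlapping enemy.
; Tick counts down a fixed cooldown, then ShootProjectile spawns the projectile, plays a sound and attack animation, and turns the tower toward the target.
; The looping animation resumes whenever the mesh stops playing.
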(event OnComponentBeginOverlap(Radius)
  (params (OverlappedComponent :type Primitive%20Component%20Object%20Reference) (OtherActor :type Actor%20Object%20Reference) (OtherComp :type Primitive%20Component%20Object%20Reference) (OtherBodyIndex :type Integer) (bFromSweep :type Boolean) (SweepResult :type Hit%20Result%20Structure%20%28by%20ref%29))
  (Utilities|IsValid (Variables|Default|GetCurrentTarget)
    (:Is%20Not%20Valid
      (if (Actor|ActorHasTag OtherActor "enemy")
        (Variables|Default|SetCurrentTarget OtherActor)))))

(event OnComponentEndOverlap(Radius)
  (params (OverlappedComponent :type Primitive%20Component%20Object%20Reference) (OtherActor :type Actor%20Object%20Reference) (OtherComp :type Primitive%20Component%20Object%20Reference) (OtherBodyIndex :type Integer))
  (if (== OtherActor (Variables|Default|GetCurrentTarget))
    (Variables|Default|SetClosestEnemy 0)
    (for _array_element (Collision|GetOverlappingActors 0 :!class /Script/Engine.Actor)
      (if (Actor|ActorHasTag _array_element "enemy")
        (Utilities|IsValid (Variables|Default|GetClosestEnemy)
          (:Is%20Valid
            (if (< (Math|Vector|Distance(Vector) (Transformation|GetActorLocation _array_element) (Transformation|GetActorLocation)) (Variables|Default|GetClosestDistance))
              (Variables|Default|SetClosestEnemy _array_element :!label _label)
              (Variables|Default|SetClosestDistance (Math|Vector|Distance(Vector) (Transformation|GetActorLocation _array_element) (Transformation|GetActorLocation)))))
          (:Is%20Not%20Valid
            (goto _label)))))
    (Variables|Default|SetCurrentTarget (Variables|Default|GetClosestEnemy))))

(event EventBeginPlay)

(event Collision|EventActorBeginOverlap
  (params (OtherActor :type Actor%20Object%20Reference)))

(event EventTick
  (params (DeltaSeconds :type Float%20%28single-precision%29))
  (if (Audio|Components|Audio|IsPlaying (Variables|Default|GetSkeletalMesh))
    _
    (else
      (Components|Animation|PlayAnimation (Variables|Default|GetSkeletalMesh) "/Game/Assets/Acid/Anim_1_GorfadaArm.Anim_1_GorfadaArm" true)))
  (bind _output_get (Variables|Default|SetShootDelay (Math|Float|Max(Float) (- (Variables|Default|GetShootDelay) DeltaSeconds) 0.0)))
  (if (== _output_get 0.0)
    (Utilities|IsValid (Variables|Default|GetCurrentTarget)
      (:Is%20Valid
        (CallFunction|ShootProjectile)))))

(fn ConstructionScript)

(fn ShootProjectile
  (bind _radius (Variables|Default|GetRadius))
  (bind _currenttarget (Variables|Default|GetCurrentTarget))
  (bind _returnvalue (Actor|GetComponentbyClass _currenttarget "/Script/Engine.SceneComponent"))
  (bind _returnvalue_2 (Transformation|GetWorldLocation _radius))
  (bind _returnvalue_3 (Transformation|GetWorldLocation _returnvalue))
  (bind _returnvalue_4 (Math|Rotator|FindLookatRotation _returnvalue_2 _returnvalue_3))
  (Game|SpawnActorfromClass "/Game/Towers/BP_AcidProjectile.BP_AcidProjectile_C" (Math|Transform|MakeTransform _returnvalue_2 "0, 0, 0" "1.000000,1.000000,1.000000") "Undefined" "MultiplyWithRoot" 0 _returnvalue 0)
  (Variables|Default|SetShootDelay 2.5)
  (Audio|PlaySoundatLocation "/Game/Assets/SFXs/Gorfada_Atk_1.Gorfada_Atk_1" _returnvalue_2 "0, 0, 0" 1.0 1.0 0.0 0 0 0 0)
  (Transformation|SetActorRotation (Math|Rotator|MakeRotator (.roll _returnvalue_4) 0.0 (.yaw _returnvalue_4)))
  (Components|Animation|PlayAnimation (Variables|Default|GetSkeletalMesh) "/Game/Assets/Acid/Anim_0_GorfadaArm.Anim_0_GorfadaArm" false))
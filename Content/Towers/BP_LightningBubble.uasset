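; BP_LightningBubble is a tower homing projectile that chains between "Enemy"-tagged actors, damaging and stunning them.
; It homes on a preset target component; each enemy overlap plays a sound and spends a bounce.
; It retargets to the first other enemy found in range, not the nearest, using AuxTarget to detect an unchanged target.
; It destroys itself when bounces, valid target or new target run out, or after a fixed lifetime.
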(event OnComponentBeginOverlap(Sphere)
  (params (OverlappedComponent :type Primitive%20Component%20Object%20Reference) (OtherActor :type Actor%20Object%20Reference) (OtherComp :type Primitive%20Component%20Object%20Reference) (OtherBodyIndex :type Integer) (bFromSweep :type Boolean) (SweepResult :type Hit%20Result%20Structure%20%28by%20ref%29))
  (if (Actor|ActorHasTag OtherActor "Enemy")
    (Game|Damage|ApplyDamage OtherActor 2e+01 0 0)
    (Audio|PlaySoundatLocation "/Game/Assets/SFXs/Cadeia_eletrica_Hit_1.Cadeia_eletrica_Hit_1" (Transformation|GetActorLocation) "0, 0, 0" 1.0 1.0 0.0 0 0 0 0)
    (bind _asbp_enemy (Utilities|Casting|CastToBP_Enemy OtherActor))
    (Default|Stun _asbp_enemy 1.0)
    (Variables|Default|SetBounces (- (Variables|Default|GetBounces) 1))
    (if (> (Variables|Default|GetBounces) 0)
      (bind _outactors (Actor|GetAllActorswithTag "Enemy"))
      (bind _array_element (Utilities|Array|ForEachLoopwithBreak _outactors :!label _label)
        (:LoopBody
          (if (!= _array_element OtherActor)
            (if (< (Math|Vector|Distance(Vector) (Transformation|GetActorLocation _array_element) (Transformation|GetActorLocation)) 8e+02)
              (bind _output_get (Variables|Components|SetHoming%20Target%20Component (Actor|GetComponentbyClass _array_element "/Script/Engine.SceneComponent")))
              (Variables|/Script/Engine.ProjectileMovementComponent|SetHomingTargetComponent (Variables|Components|GetProjectileMovement) _output_get)
              (goto _label Break))))
        (:Completed
          (if (== (Variables|Default|GetAuxTarget) (Variables|Components|GetHoming%20Target%20Component))
            (Actor|DestroyActor)
            (else
              (Variables|Default|SetAuxTarget (Variables|Components|GetHoming%20Target%20Component))))))
      (else
        (Actor|DestroyActor)))))

(event EventBeginPlay
  (bind _homing_target_component (Variables|Components|GetHoming%20Target%20Component))
  (Variables|/Script/Engine.ProjectileMovementComponent|SetHomingTargetComponent (Variables|Components|GetProjectileMovement) _homing_target_component)
  (Variables|Default|SetAuxTarget _homing_target_component)
  (Utilities|FlowControl|Delay 1e+01)
  (Actor|DestroyActor))

(event Collision|EventActorBeginOverlap
  (params (OtherActor :type Actor%20Object%20Reference)))

(event EventTick
  (params (DeltaSeconds :type Float%20%28single-precision%29))
  (Utilities|IsValid (Variables|Components|GetHoming%20Target%20Component)
    (:Is%20Not%20Valid
      (Actor|DestroyActor))))

(fn ConstructionScript)
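; BP_FireBubble is a homing tower projectile that explodes on enemies for area damage.
; On spawn it homes on its assigned target component, destroying itself after a fixed lifetime or when that target becomes invalid.
; When its sphere overlaps an Enemy-tagged actor, it plays effects, damages nearby enemies, then destroys itself.
; The blast finds victims by distance-checking every Enemy-tagged actor rather than using a radial damage or overlap query.
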(event OnComponentBeginOverlap(Sphere)
  (params (OverlappedComponent :type Primitive%20Component%20Object%20Reference) (OtherActor :type Actor%20Object%20Reference) (OtherComp :type Primitive%20Component%20Object%20Reference) (OtherBodyIndex :type Integer) (bFromSweep :type Boolean) (SweepResult :type Hit%20Result%20Structure%20%28by%20ref%29))
  (bind _returnvalue (Transformation|GetActorLocation))
  (if (Actor|ActorHasTag OtherActor "Enemy")
    (Niagara|SpawnSystematLocation "/Game/Towers/P_Explosion.P_Explosion" (Math|Vector|MakeVector (.x _returnvalue) (.y _returnvalue) (+ (.z _returnvalue) 2e+02)))
    (Audio|PlaySoundatLocation "/Game/Assets/SFXs/Botano_Butano_Hit_1.Botano_Butano_Hit_1" (Transformation|GetActorLocation) "0, 0, 0" 1.0 1.0 0.0 0 0 0 0)
    (bind _outactors (Actor|GetAllActorswithTag "Enemy"))
    (for _array_element _outactors
      (if (< (Math|Vector|Distance(Vector) (Transformation|GetActorLocation _array_element) (Transformation|GetActorLocation)) 8e+02)
        (Game|Damage|ApplyDamage _array_element 5e+01 0 0)))
    (Actor|DestroyActor)))

(event EventBeginPlay
  (Variables|/Script/Engine.ProjectileMovementComponent|SetHomingTargetComponent (Variables|Components|GetProjectileMovement) (Variables|Components|GetHoming%20Target%20Component))
  (Utilities|FlowControl|Delay 1e+01)
  (Actor|DestroyActor))

(event Collision|EventActorBeginOverlap
  (params (OtherActor :type Actor%20Object%20Reference)))

(event EventTick
  (params (DeltaSeconds :type Float%20%28single-precision%29))
  (Utilities|IsValid (Variables|Components|GetHoming%20Target%20Component)
    (:Is%20Not%20Valid
      (Actor|DestroyActor))))

(fn ConstructionScript)
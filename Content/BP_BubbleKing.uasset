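; BP_BubbleKing is a damageable actor with a health bar widget in the world.
; Health starts at InitialHealth and drops with any damage, clamped at zero, with no death handling.
; Each tick pushes the health fraction into the WB_HealthBar progress bar.
; It also tilts the widget toward the player camera using look-at roll and pitch, with yaw locked at 180 degrees.
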(event EventBeginPlay
  (Variables|Combat|SetHealth (Variables|Combat|GetInitialHealth)))

(event Collision|EventActorBeginOverlap
  (params (OtherActor :type Actor%20Object%20Reference)))

(event EventTick
  (params (DeltaSeconds :type Float%20%28single-precision%29))
  (bind _returnvalue (Game|GetPlayerCameraManager 0))
  (bind _healthbarwidget (Variables|Default|GetHealthBarWidget))
  (bind _returnvalue_2 (Transformation|GetWorldLocation _healthbarwidget))
  (bind _transformcomponent (Variables|/Script/Engine.PlayerCameraManager|GetTransformComponent _returnvalue))
  (bind _returnvalue_3 (Transformation|GetWorldLocation _transformcomponent))
  (bind _returnvalue_4 (Math|Rotator|FindLookatRotation _returnvalue_2 _returnvalue_3))
  ;[0.15 0.15 0.15 0.5] Update health bar widget.
  (bind _aswb_health_bar (Utilities|Casting|CastToWB_HealthBar (UserInterface|GetWidget _healthbarwidget)))
  (Progress|SetPercent (Variables|/Game/TowerDefense/WB_HealthBar.WB_HealthBar_C|GetProgressBar _aswb_health_bar) (/ (Variables|Combat|GetHealth) (Variables|Combat|GetInitialHealth)))
  (Transformation|SetWorldRotation _healthbarwidget (Math|Rotator|MakeRotator (.roll _returnvalue_4) (.pitch _returnvalue_4) 1.8e+02) false false))

(event Game|Damage|EventAnyDamage
  (params (Damage :type Float%20%28single-precision%29) (DamageType :type Damage%20Type%20Object%20Reference) (InstigatedBy :type Controller%20Object%20Reference) (DamageCauser :type Actor%20Object%20Reference))
  (Variables|Combat|SetHealth (Math|Float|Max(Float) (- (Variables|Combat|GetHealth) Damage) 0.0)))

(fn ConstructionScript)
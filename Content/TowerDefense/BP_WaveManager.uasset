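; Tower defense wave manager that spawns enemies on a repeating countdown at the start of a referenced Path and moves them along it.
; Each Tick, it asks living enemies for their advanced distance, converts that to a path location and turns them toward it.
; Dead enemies and those reaching the path's end go into an expired list, destroyed after the loop to avoid modifying the array mid-iteration.
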(event EventBeginPlay
  (bind _path (Variables|Default|GetPath)
    (:then
      (bind _length (Default|GetLength _path))
      (Variables|Default|SetPathLength _length))
    (:else)))

(event Collision|EventActorBeginOverlap
  (params (OtherActor :type Actor%20Object%20Reference)))

(event EventTick
  (params (DeltaSeconds :type Float%20%28single-precision%29))
  (CallFunction|UpdateWave DeltaSeconds))

(fn ConstructionScript)

(fn UpdateWave
  (params (DeltaSeconds :type Float%20%28double-precision%29))
  (Utilities|FlowControl|Sequence
    (:then_0
      ;[0.15 0.15 0.15 0.5] Spawn a new enemy.
      (bind _output_get (Variables|Default|SetTimeUntilEnemy (- (Variables|Default|GetTimeUntilEnemy) DeltaSeconds)))
      (if (< _output_get 0.0)
        (Variables|Default|SetTimeUntilEnemy (Variables|Default|GetSpawnCountdown))
        (bind _location (Default|GetLocation (Variables|Default|GetPath) 0.0))
        (bind _returnvalue (Game|SpawnActorfromClass "/Game/TowerDefense/BP_Enemy.BP_Enemy_C" (Math|Transform|MakeTransform _location "0, 0, 0" "1.000000,1.000000,1.000000") "Undefined" "MultiplyWithRoot" 0 0))
        (Utilities|Array|Add (Variables|Default|GetEnemies) _returnvalue)))
    (:then_1
      (CallFunction|AdvanceEnemies DeltaSeconds)
      (CallFunction|CleanUpEnemies))))

(fn AdvanceEnemies
  (params (DeltaSeconds :type Float%20%28double-precision%29))
  (for _array_element (Variables|Default|GetEnemies)
    (if (Variables|/Game/TowerDefense/BP_Enemy.BP_Enemy_C|GetIsAlive _array_element)
      (bind _distance (Default|Advance _array_element DeltaSeconds))
      (if (< _distance (Variables|Default|GetPathLength))
        (bind _location (Default|GetLocation (Variables|Default|GetPath) _distance))
        (Transformation|SetActorLocationAndRotation _array_element _location (Math|Rotator|FindLookatRotation (Transformation|GetActorLocation _array_element) _location))
        (else
          (|AddToExpiredEnemies2 _array_element)))
      (else
        (|AddToExpiredEnemies1 _array_element)))))

(fn CleanUpEnemies
  (bind _expiredenemies (Variables|Default|GetExpiredEnemies))
  (for _array_element _expiredenemies
    (Utilities|Array|RemoveItem (Variables|Default|GetEnemies) _array_element)
    (Actor|DestroyActor _array_element))
  (Utilities|Array|Clear _expiredenemies))
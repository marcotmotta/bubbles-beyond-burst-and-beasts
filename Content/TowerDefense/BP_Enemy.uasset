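; BP_Enemy is a tower defense enemy that tracks its life, speed and distance travelled.
; BeginPlay copies the initial life and speed into the working values.
; Advance adds speed times delta seconds to the distance and returns it, while TakeDamage subtracts damage from life, floors it at zero and returns it.
; It has no active Tick and never moves itself, so both functions rely on outside callers.
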(event EventBeginPlay
  (Variables|Default|SetLife (Variables|Default|GetInitialLife))
  (Variables|Default|SetSpeed (Variables|Default|GetInitialSpeed)))

(event Collision|EventActorBeginOverlap
  (params (OtherActor :type Actor%20Object%20Reference)))

(event EventTick
  (params (DeltaSeconds :type Float%20%28single-precision%29)))

(fn ConstructionScript)

(fn Advance
  (params (DeltaSeconds :type Float%20%28double-precision%29))
  (bind _output_get (Variables|Default|SetDistance (+ (* DeltaSeconds (Variables|Default|GetSpeed)) (Variables|Default|GetDistance))))
  (return _output_get))

(fn TakeDamage
  (params (Damage :type Float%20%28double-precision%29))
  (bind _output_get (Variables|Default|SetLife (Math|Float|Max(Float) (- (Variables|Default|GetLife) Damage) 0.0)))
  (return _output_get))
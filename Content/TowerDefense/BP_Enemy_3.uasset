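; BP_Enemy_3 is an enemy Blueprint for the tower defense game that supplies its own attack presentation.
; PlayAttack plays a one-shot Ignacio arm animation on the skeletal mesh and an Ignacio attack sound at the actor's location.
; The event graph holds only disabled stub events, and the construction script just calls its parent.
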(event EventBeginPlay
  (|CallParentFunction) ; This node is disabled and will not be called.\nDrag off pins to build functionality.
)

(event Collision|EventActorBeginOverlap
  (params (OtherActor :type Actor%20Object%20Reference))
  (|CallParentFunction OtherActor) ; This node is disabled and will not be called.\nDrag off pins to build functionality.
)

(event EventTick
  (params (DeltaSeconds :type Float%20%28single-precision%29))
  (|CallParentFunction DeltaSeconds) ; This node is disabled and will not be called.\nDrag off pins to build functionality.
)

(fn ConstructionScript
  (|CallParentFunction))

(fn PlayAttack
  (Components|Animation|PlayAnimation (Variables|Default|GetSkeletalMesh) "/Game/Assets/Ignacio/Anim_1_IgnacioArm.Anim_1_IgnacioArm" false)
  (Audio|PlaySoundatLocation "/Game/Assets/SFXs/Ignacio_Atk_1.Ignacio_Atk_1" (Transformation|GetActorLocation) "0, 0, 0" 1.0 1.0 0.0 0 0 0 0))
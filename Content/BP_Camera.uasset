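; BP_Camera is a player-controlled camera actor that pans horizontally with WASD and zooms with the mouse wheel.
; Key presses and releases add or subtract axis vectors from CamMovement, which Tick normalizes, scales by CamSpeed and adds to the actor location.
; The step is per frame without delta time, so pan speed depends on frame rate.
; The mouse wheel changes the spring arm length within clamped limits to zoom.
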(event EventBeginPlay)

(event Collision|EventActorBeginOverlap
  (params (OtherActor :type Actor%20Object%20Reference)))

(event EventTick
  (params (DeltaSeconds :type Float%20%28single-precision%29))
  (Transformation|SetActorLocation (+ (Transformation|GetActorLocation) (* (Math|Vector|Normalize (Variables|Default|GetCamMovement)) (Variables|Default|GetCamSpeed))) false false))

(event Input|ActionEvents|InputActiona
  (params (Key :type Key%20Structure :default "None"))
  ;[0.15 0.15 0.15 0.5] Input for camera movement
  (:Pressed
    (Variables|Default|SetCamMovement (- (Variables|Default|GetCamMovement) "0.000000,1.000000,0.000000")))
  (:Released
    (Variables|Default|SetCamMovement (+ (Variables|Default|GetCamMovement) "0.000000,1.000000,0.000000"))))

(event Input|ActionEvents|InputActionw
  (params (Key :type Key%20Structure :default "None"))
  ;[0.15 0.15 0.15 0.5] Input for camera movement
  (:Pressed
    (Variables|Default|SetCamMovement (+ (Variables|Default|GetCamMovement) "1.000000,0.000000,0.000000")))
  (:Released
    (Variables|Default|SetCamMovement (- (Variables|Default|GetCamMovement) "1.000000,0.000000,0.000000"))))

(event Input|ActionEvents|InputActiond
  (params (Key :type Key%20Structure :default "None"))
  ;[0.15 0.15 0.15 0.5] Input for camera movement
  (:Pressed
    (Variables|Default|SetCamMovement (+ (Variables|Default|GetCamMovement) "0.000000,1.000000,0.000000")))
  (:Released
    (Variables|Default|SetCamMovement (- (Variables|Default|GetCamMovement) "0.000000,1.000000,0.000000"))))

(event Input|ActionEvents|InputActions
  (params (Key :type Key%20Structure :default "None"))
  ;[0.15 0.15 0.15 0.5] Input for camera movement
  (:Pressed
    (Variables|Default|SetCamMovement (- (Variables|Default|GetCamMovement) "1.000000,0.000000,0.000000")))
  (:Released
    (Variables|Default|SetCamMovement (+ (Variables|Default|GetCamMovement) "1.000000,0.000000,0.000000"))))

(event Input|MouseEvents|MouseWheelAxis
  (params (AxisValue :type Float%20%28single-precision%29))
  ;[0.15 0.15 0.15 0.5] Input for camera movement
  (Variables|/Script/Engine.SpringArmComponent|SetTargetArmLength (Variables|Default|GetSpringArm) (Math|Float|Clamp(Float) (+ (* AxisValue -1e+02) (Variables|/Script/Engine.SpringArmComponent|GetTargetArmLength (Variables|Default|GetSpringArm))) 1e+03 3e+03)))

(fn ConstructionScript)